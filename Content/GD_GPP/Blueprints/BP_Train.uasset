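; BP_Train is a moving train hazard that launches or kills the third-person player character on contact.
; Every tick it adds a constant physics force along the train mesh's forward vector, applied as an acceleration change so mass is ignored.
; A hit on the mesh calls PropulsedByATrain on the character, while overlapping the separate Destruction component calls Killed.
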(event OnComponentHit(SM_Train)
  (params (HitComponent :type Primitive%20Component%20Object%20Reference) (OtherActor :type Actor%20Object%20Reference) (OtherComp :type Primitive%20Component%20Object%20Reference) (NormalImpulse :type Vector :default "0, 0, 0") (Hit :type Hit%20Result%20Structure%20%28by%20ref%29))
  (bind _asbp_third_person_character (Utilities|Casting|CastToBP_ThirdPersonCharacter OtherActor))
  (Default|PropulsedbyATrain _asbp_third_person_character))

(event OnComponentBeginOverlap(Destruction)
  (params (OverlappedComponent :type Primitive%20Component%20Object%20Reference) (OtherActor :type Actor%20Object%20Reference) (OtherComp :type Primitive%20Component%20Object%20Reference) (OtherBodyIndex :type Integer) (bFromSweep :type Boolean) (SweepResult :type Hit%20Result%20Structure%20%28by%20ref%29))
  (bind _asbp_third_person_character (Utilities|Casting|CastToBP_ThirdPersonCharacter OtherActor))
  (Default|Killed _asbp_third_person_character))

(event EventTick
  (params (DeltaSeconds :type Float%20%28single-precision%29))
  (Physics|AddForce (Variables|Default|GetSM_Train) (* (Math|Vector|GetForwardVector (Variables|Default|GetSM_Train)) 3e+05) "None" true))

(fn ConstructionScript)