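; BP_Dummy2 is an actor carrying costume props (cowboy hat, two guns, two bananas) that transfer to the player on touch.
; When BP_PlayerMerge overlaps its Box, each static mesh component attaches to a named socket on the player's mesh, snapping location and keeping relative rotation and scale.
; The components themselves are re-parented, with no spawning, detaching or guard against repeat overlaps.
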(event OnComponentBeginOverlap(Box)
  (params (OverlappedComponent :type Primitive%20Component%20Object%20Reference) (OtherActor :type Actor%20Object%20Reference) (OtherComp :type Primitive%20Component%20Object%20Reference) (OtherBodyIndex :type Integer) (bFromSweep :type Boolean) (SweepResult :type Hit%20Result%20Structure%20%28by%20ref%29))
  (bind _asbp_player_merge (Utilities|Casting|CastToBP_PlayerMerge OtherActor))
  (Transformation|AttachComponentToComponent (Variables|Default|GetSM_CowboyHat) (Variables|/Script/Engine.Character|GetMesh _asbp_player_merge) "Kz_HairSocket" "SnapToTarget" "KeepRelative" "KeepRelative" true)
  (Transformation|AttachComponentToComponent (Variables|Default|GetSM_Gun) (Variables|/Script/Engine.Character|GetMesh _asbp_player_merge) "Kz_ArmRSocket" "SnapToTarget" "KeepRelative" "KeepRelative" true)
  (Transformation|AttachComponentToComponent (Variables|Default|GetSM_Gun1) (Variables|/Script/Engine.Character|GetMesh _asbp_player_merge) "Kz_ArmLSocket" "SnapToTarget" "KeepRelative" "KeepRelative" true)
  (Transformation|AttachComponentToComponent (Variables|Default|GetSM_Banane) (Variables|/Script/Engine.Character|GetMesh _asbp_player_merge) "Kz_Banana1" "SnapToTarget" "KeepRelative" "KeepRelative" true)
  (Transformation|AttachComponentToComponent (Variables|Default|GetSM_Banane1) (Variables|/Script/Engine.Character|GetMesh _asbp_player_merge) "Kz_Banana2" "SnapToTarget" "KeepRelative" "KeepRelative" true))

(event Collision|EventActorBeginOverlap
  (params (OtherActor :type Actor%20Object%20Reference)))

(event EventTick
  (params (DeltaSeconds :type Float%20%28single-precision%29)))

(fn ConstructionScript)