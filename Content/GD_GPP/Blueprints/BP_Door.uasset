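; BP_Door is a breakable door that players open by damaging it until its life runs out.
; OnHit subtracts damage from its life, then calls ResetDoor on the hitting player after a short delay.
; The lethal hit, guarded by DoOnce, disables the mesh's collision, plays a chest sound and starts a timeline.
; The timeline, remapped through a float curve, swings the mesh in yaw from its initial rotation.
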(event Custom|OnHit
  (params (Damage :type Float%20%28double-precision%29) (Player :type BP%20Player%20Merge%20Object%20Reference))
  ;[1 0 0 0.33] On Hit
  (if (<= (- (Variables|Default|GetCurrentLife) Damage) 0.0)
    (Utilities|FlowControl|DoOnce false
      (:Completed
        (Collision|SetCollisionEnabled (Variables|Default|GetSM_Module_Strongbox_Cylinder_003) "NoCollision")
        (CallFunction|Animation)))
    (else
      (Variables|Default|SetCurrentLife (- (Variables|Default|GetCurrentLife) Damage))))
  (Utilities|FlowControl|Delay 0.5)
  (Default|ResetDoor Player))

(event Custom|Animation
  (bind _defaultrotation (Variables|Animation|GetDefaultRotation))
  ;[0 0.5736 1 0.33] Animation
  (Audio|PlaySound2D "/Game/GD_GPP/Sound/Treasure_Chest_Sound_Effect.Treasure_Chest_Sound_Effect" 1.0 1.0 0.0 0 0)
  (bind _newtrack_0 (Timeline|T_Open PlayFromStart)
    (:Update
      (Transformation|SetWorldRotation (Variables|Default|GetSM_Module_Strongbox_Cylinder_003) (Math|Rotator|Lerp(Rotator) (Math|Rotator|MakeRotator (.roll _defaultrotation) (.pitch _defaultrotation) (.yaw _defaultrotation)) (Math|Rotator|MakeRotator (.roll _defaultrotation) (.pitch _defaultrotation) (+ (.yaw _defaultrotation) (.yaw (Variables|Animation|GetRotationMax)))) (Math|Curves|GetFloatValue (Variables|Animation|GetFloatCurve) _newtrack_0)) false false))))

(event EventBeginPlay
  (Variables|Default|SetCurrentLife (Variables|Default|GetMaxLife))
  (Variables|Animation|SetDefaultRotation (Transformation|GetWorldRotation (Variables|Default|GetSM_Module_Strongbox_Cylinder_003))))

(fn ConstructionScript)