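; A train hazard that drives forward, launches players it hits, and destroys characters that enter its destruction zone.
; A sound plays at spawn, and Tick pushes the train mesh along its forward vector with a mass-independent force.
; Mesh hits call PropulsedByATrain on BP_PlayerMerge, while Destruction overlaps call Killed on it.
; Overlapping BP_CharaTest actors are destroyed with a Niagara poof explosion, removed after a short delay.
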(event OnComponentHit(SM_Train)
  (params (HitComponent :type Primitive%20Component%20Object%20Reference) (OtherActor :type Actor%20Object%20Reference) (OtherComp :type Primitive%20Component%20Object%20Reference) (NormalImpulse :type Vector :default "0, 0, 0") (Hit :type Hit%20Result%20Structure%20%28by%20ref%29))
  (bind _asbp_player_merge (Utilities|Casting|CastToBP_PlayerMerge OtherActor))
  (Default|PropulsedbyATrain _asbp_player_merge))

(event OnComponentBeginOverlap(Destruction)
  (params (OverlappedComponent :type Primitive%20Component%20Object%20Reference) (OtherActor :type Actor%20Object%20Reference) (OtherComp :type Primitive%20Component%20Object%20Reference) (OtherBodyIndex :type Integer) (bFromSweep :type Boolean) (SweepResult :type Hit%20Result%20Structure%20%28by%20ref%29))
  (bind _asbp_player_merge (Utilities|Casting|CastToBP_PlayerMerge OtherActor)
    (:then
      (Default|Killed _asbp_player_merge))
    (:CastFailed
      (bind _asbp_chara_test (Utilities|Casting|CastToBP_CharaTest OtherActor))
      (bind _returnvalue (Niagara|SpawnSystematLocation "/Game/GA/FX/NS_Poof_Explosion.NS_Poof_Explosion" (Transformation|GetWorldLocation (Variables|/Script/Engine.Character|GetMesh _asbp_chara_test)) "0, 0, 0" "3.000000,3.000000,3.000000"))
      (Actor|DestroyActor _asbp_chara_test)
      (Utilities|FlowControl|Delay 2.0)
      (Components|DestroyComponent _returnvalue))))

(event EventBeginPlay
  (Audio|PlaySound2D "/Game/GD_GPP/Sound/Train_sound_effect___no_copyright_.Train_sound_effect___no_copyright_" 1.0 1.0 0.0 0 0))

(event EventTick
  (params (DeltaSeconds :type Float%20%28single-precision%29))
  (Physics|AddForce (Variables|Default|GetSM_Train) (* (Math|Vector|GetForwardVector (Variables|Default|GetSM_Train)) 3e+05) "None" true))

(fn ConstructionScript)