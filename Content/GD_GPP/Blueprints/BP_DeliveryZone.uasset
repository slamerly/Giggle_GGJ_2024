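; A delivery zone trigger where a player carrying money cashes in their wallet for score.
; When a BP_PlayerMerge with HaveMoney overlaps the box, it destroys every carried wallet actor and clears the money flag.
; DeliverMoney recursively walks the socket index down to zero, sending each stored score to BP_ThirdPersonGameMode's UpdateScore, then empties the wallet arrays.
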(event OnComponentBeginOverlap(Box)
  (params (OverlappedComponent :type Primitive%20Component%20Object%20Reference) (OtherActor :type Actor%20Object%20Reference) (OtherComp :type Primitive%20Component%20Object%20Reference) (OtherBodyIndex :type Integer) (bFromSweep :type Boolean) (SweepResult :type Hit%20Result%20Structure%20%28by%20ref%29))
  (bind _asbp_player_merge (Utilities|Casting|CastToBP_PlayerMerge OtherActor))
  (if (Variables|/Game/GD_GPP/Blueprints/BP_PlayerMerge.BP_PlayerMerge_C|GetHaveMoney _asbp_player_merge)
    (bind _output_get (Variables|Default|SetPlayerMerge _asbp_player_merge))
    (for _array_element (Variables|/Game/GD_GPP/Blueprints/BP_PlayerMerge.BP_PlayerMerge_C|GetWalletArrey _output_get)
      (Actor|DestroyActor _array_element))
    (CallFunction|DeliverMoney)
    (Variables|/Game/GD_GPP/Blueprints/BP_PlayerMerge.BP_PlayerMerge_C|SetHaveMoney (Variables|Default|GetPlayerMerge) false)))

(event Custom|DeliverMoney
  (bind _playermerge (Variables|Default|GetPlayerMerge))
  (bind _playermerge_2 (Variables|Default|GetPlayerMerge))
  (if (> (Variables|/Game/GD_GPP/Blueprints/BP_PlayerMerge.BP_PlayerMerge_C|GetIndexSocket _playermerge_2) 0)
    (bind _output_get (Variables|/Game/GD_GPP/Blueprints/BP_PlayerMerge.BP_PlayerMerge_C|SetIndexSocket _playermerge (- (Variables|/Game/GD_GPP/Blueprints/BP_PlayerMerge.BP_PlayerMerge_C|GetIndexSocket _playermerge) 1)))
    (bind _asbp_third_person_game_mode (Utilities|Casting|CastToBP_ThirdPersonGameMode (Game|GetGameMode)))
    (Default|UpdateScore _asbp_third_person_game_mode (Pawn|GetLocalViewingPlayerController (Variables|Default|GetPlayerMerge)) (Utilities|Array|Get(acopy) (Variables|/Game/GD_GPP/Blueprints/BP_PlayerMerge.BP_PlayerMerge_C|GetWalletScore _playermerge) _output_get))
    (CallFunction|DeliverMoney)
    (else
      (Utilities|Array|Clear (Variables|/Game/GD_GPP/Blueprints/BP_PlayerMerge.BP_PlayerMerge_C|GetWalletArrey _playermerge_2))
      (Utilities|Array|Clear (Variables|/Game/GD_GPP/Blueprints/BP_PlayerMerge.BP_PlayerMerge_C|GetWalletType _playermerge_2))
      (Utilities|Array|Clear (Variables|/Game/GD_GPP/Blueprints/BP_PlayerMerge.BP_PlayerMerge_C|GetWalletScore _playermerge_2)))))

(fn ConstructionScript)