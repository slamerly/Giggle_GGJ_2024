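; BP_CharaTest is a test character with logic for endless random roaming, though nothing starts it.
; RandomRoam uses AI MoveTo toward a random reachable point around the character, then calls itself again on success or failure.
; BeginPlay is empty, and the nodes that would apply a random mesh material and start roaming are disconnected, so they never run.
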(event Custom|Random%20Roam
  (AI|AIMoveTo self (.RandomLocation (AI|Navigation|GetRandomReachablePointinRadius (Transformation|GetActorLocation) 1e+03 0 0)) 0 5.0 false
    (:OnSuccess
      (CallFunction|RandomRoam))
    (:OnFail
      (CallFunction|RandomRoam))))

(event EventBeginPlay)

(fn ConstructionScript)