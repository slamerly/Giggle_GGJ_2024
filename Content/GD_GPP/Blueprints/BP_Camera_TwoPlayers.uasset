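; Shared camera actor that keeps two players framed by following their midpoint and zooming with their separation.
; After a short startup delay it caches all Characters, then a gated Tick works on the first two.
; A box component moves to the midpoint, and the spring arm eases toward it at fixed height with an offset.
; Arm length interpolates toward a clamped value derived from player distance.
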(event Custom|Set%20Longest%20Distance%20Between%20Players
  ;[1 1 1] Take the longest distance between players
  (Variables|Default|SetLongest%20Distance (- (Math|Float|Max(Float) (Transformation|GetDistanceTo (Utilities|Array|Get(acopy) (Variables|Default|GetCharacters)) (Utilities|Array|Get(acopy) (Variables|Default|GetCharacters) 1)) 0.0) 1.3e+03)))

(event Custom|Set%20Center%20Point
  ;[1 1 1] Set Center Point Between Players
  (Variables|Default|SetCenter%20Position (/ (+ (Transformation|GetActorLocation (Utilities|Array|Get(acopy) (Variables|Default|GetCharacters))) (Transformation|GetActorLocation (Utilities|Array|Get(acopy) (Variables|Default|GetCharacters) 1))) "2.000000,2.000000,2.000000")))

(event Custom|Camera%20Zoom
  (bind _springarm (Variables|Default|GetSpringArm))
  ;[1 1 1] Camera Zoom
  (Variables|/Script/Engine.SpringArmComponent|SetTargetArmLength _springarm (Math|Interpolation|FInterpTo (Variables|/Script/Engine.SpringArmComponent|GetTargetArmLength _springarm) (Math|Float|Max(Float) (Math|Float|Min(Float) (Variables|Default|GetLongest%20Distance) 8e+02) -5e+02) (Variables|Default|GetDelta%20Time) 1.0)))

(event Custom|Set%20Box%20Position
  ;[1 1 1] Set Box Position (Debug Camera Position)
  (Transformation|SetWorldLocation (Variables|Default|GetBox) (Variables|Default|GetCenter%20Position) false false))

(event Custom|Set%20Camera%20Position
  (bind _box (Variables|Default|GetBox))
  (bind _returnvalue (Transformation|GetWorldLocation _box))
  (bind (_x _y) (Math|Vector|BreakVector _returnvalue))
  ;[1 1 1] Set Camera Position
  (Variables|Default|SetCamera%20Y%20Pos (Math|Interpolation|FInterpTo (Variables|Default|GetCamera%20Y%20Pos) (- _x (Variables|Default|GetY%20Offset)) (Variables|Default|GetDelta%20Time) 0.5))
  (Variables|Default|SetCamera%20X%20Pos (Math|Interpolation|FInterpTo (Variables|Default|GetCamera%20X%20Pos) _y (Variables|Default|GetDelta%20Time) 0.5))
  (Transformation|SetWorldLocation (Variables|Default|GetSpringArm) (Math|Vector|MakeVector (Variables|Default|GetCamera%20Y%20Pos) (Variables|Default|GetCamera%20X%20Pos) (.Z (Math|Vector|BreakVector (Variables|Default|GetCamera%20Start%20Pos)))) false false))

(event EventBeginPlay
  (bind _springarm (Variables|Default|GetSpringArm))
  (bind _returnvalue (Transformation|GetWorldLocation _springarm))
  (bind (_x _y) (Math|Vector|BreakVector _returnvalue))
  (Utilities|FlowControl|Sequence
    (:then_0
      (Utilities|FlowControl|Delay 0.5)
      (bind _outactors (Actor|GetAllActorsOfClass "/Script/Engine.Character"))
      (bind _output_get (Variables|Default|SetCharacters _outactors))
      (Development|PrintString (Utilities|String|ToString(Integer) (Utilities|Array|Length _output_get))))
    (:then_1
      (Variables|Default|SetCamera%20Y%20Pos _y)
      (Variables|Default|SetCamera%20X%20Pos _x)
      (Variables|Default|SetCamera%20Start%20Pos (Math|Vector|MakeVector 0.0 0.0 (.Z (Math|Vector|BreakVector (Transformation|GetActorLocation))))))
    (:then_2
      (Utilities|FlowControl|Delay 0.5)
      (Utilities|FlowControl|Gate true) ; enters at Open
    )))

(event EventTick
  (params (DeltaSeconds :type Float%20%28single-precision%29))
  (Utilities|FlowControl|Gate true
    (:Exit
      (Variables|Default|SetDelta%20Time DeltaSeconds)
      (Utilities|IsValid (Utilities|Array|Get(acopy) (Variables|Default|GetCharacters))
        (:Is%20Valid
          (Utilities|IsValid (Utilities|Array|Get(acopy) (Variables|Default|GetCharacters) 1)
            (:Is%20Valid
              (CallFunction|SetLongestDistanceBetweenPlayers)
              (CallFunction|SetCenterPoint)
              (CallFunction|CameraZoom)
              (CallFunction|SetCameraPosition)
              (CallFunction|SetBoxPosition))))))))

(fn ConstructionScript)