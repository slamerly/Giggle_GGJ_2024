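; Breakable strongbox that takes damage from players and, once its life runs out, opens to scatter money wallets.
; OnHit lowers life or triggers the one-time opening, calling ResetCoffre on the attacking player after a short delay.
; A timeline remapped through a float curve swings the door's yaw with collision disabled.
; When it finishes, collision returns and a random number of BP_MoneyWallet actors spawn at random reachable points around SpawnPoint.
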(event Custom|OnHit
  (params (Damage :type Float%20%28double-precision%29) (Player :type BP%20Player%20Merge%20Object%20Reference))
  ;[1 0 0 0.33] On Hit
  (if (<= (- (Variables|Default|GetCurrentLife) Damage) 0.0)
    (Utilities|FlowControl|DoOnce false
      (:Completed
        (Collision|SetCollisionEnabled (Variables|Default|GetSM_Strongbox_Door) "NoCollision")
        (CallFunction|Animation)))
    (else
      (Variables|Default|SetCurrentLife (- (Variables|Default|GetCurrentLife) Damage))))
  (Utilities|FlowControl|Delay 0.5)
  (Default|ResetCoffre Player))

(event Custom|Animation
  (bind _defaultrotation (Variables|Animation|GetDefaultRotation))
  ;[0 0.5736 1 0.33] Animation
  (bind _newtrack_0 (Timeline|T_Open PlayFromStart)
    (:Update
      (Transformation|SetWorldRotation (Variables|Default|GetSM_Strongbox_Door) (Math|Rotator|Lerp(Rotator) (Math|Rotator|MakeRotator (.roll _defaultrotation) (.pitch _defaultrotation) (.yaw _defaultrotation)) (Math|Rotator|MakeRotator (.roll _defaultrotation) (.pitch _defaultrotation) (+ (.yaw _defaultrotation) (.yaw (Variables|Animation|GetRotationMax)))) (Math|Curves|GetFloatValue (Variables|Animation|GetFloatCurve) _newtrack_0)) false false))
    (:Finished
      (Collision|SetCollisionEnabled (Variables|Default|GetSM_Strongbox_Door) "QueryAndPhysics")
      (CallFunction|SpawnWallet))))

(event Custom|SpawnWallet
  ;[0.1928 1 0 0.33] Spawn
  (bind _output_get (Variables|Spawn|SetNbWalletToSpawn (Math|Random|RandomIntegerinRange (Variables|Spawn|GetNbMinWalletSpawn) (Variables|Spawn|GetNbMaxWalletSpawn))))
  (while (> _output_get 0)
    (Game|SpawnActorfromClass "/Game/GD_GPP/Blueprints/BP_MoneyWallet.BP_MoneyWallet_C" (Math|Transform|MakeTransform (.RandomLocation (AI|Navigation|GetRandomReachablePointinRadius (Transformation|GetWorldLocation (Variables|Default|GetSpawnPoint)) (Variables|Spawn|GetRadiusSpawn) 0 0)) (Math|Rotator|MakeRotator 0.0 0.0 (Math|Random|RandomFloatinRange 0.0 3.6e+02)) "1.000000,1.000000,1.000000") "Undefined" "MultiplyWithRoot" 0 0)
    (Math|Integer|DecrementInt (Variables|Spawn|GetNbWalletToSpawn))))

(event EventBeginPlay
  (Variables|Default|SetCurrentLife (Variables|Default|GetMaxLife))
  (Variables|Animation|SetDefaultRotation (Transformation|GetWorldRotation (Variables|Default|GetSM_Strongbox_Door))))

(fn ConstructionScript)