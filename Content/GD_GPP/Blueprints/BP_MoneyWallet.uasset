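; BP_MoneyWallet is a money pickup that the player collects by touching it.
; On BeginPlay it sets mesh and value from its money type (coin pile, bills or money bag), picking a random type if none is set.
; A timeline and float curve animate its position between the start point and an AddHauteur offset.
; Overlap with BP_PlayerMerge destroys the collision to prevent repeat triggers, then passes the wallet to the player's CollectWallet.
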(event OnComponentBeginOverlap(Collision)
  (params (OverlappedComponent :type Primitive%20Component%20Object%20Reference) (OtherActor :type Actor%20Object%20Reference) (OtherComp :type Primitive%20Component%20Object%20Reference) (OtherBodyIndex :type Integer) (bFromSweep :type Boolean) (SweepResult :type Hit%20Result%20Structure%20%28by%20ref%29))
  (bind _asbp_player_merge (Utilities|Casting|CastToBP_PlayerMerge OtherActor))
  (Components|DestroyComponent (Variables|Default|GetCollision))
  (Default|CollectWallet _asbp_player_merge self))

(event EventBeginPlay
  (CallFunction|Initialisation)
  (Variables|Animation|SetStartPosition (Transformation|GetActorLocation))
  (bind _newtrack_0 (Timeline|T_Animation PlayFromStart)
    (:Update
      (Transformation|SetActorLocation (Math|Vector|Lerp(Vector) (Variables|Animation|GetStartPosition) (+ (Variables|Animation|GetStartPosition) (Variables|Animation|GetAddHauteur)) (Math|Curves|GetFloatValue (Variables|Animation|GetCurveAnimation) _newtrack_0)) false false))))

(fn ConstructionScript)

(fn Initialisation
  (if (Utilities|Enum|Equal(Enum) (Variables|Default|GetTypeOfMoney) "NewEnumerator3")
    (Variables|Default|SetTypeOfMoney (.OutItem (Utilities|Array|Random (Variables|Default|GetEnum_Money)))))
  (switch Utilities|FlowControl|Switch|SwitchonEnum_CollectibleMoney (Variables|Default|GetTypeOfMoney)
    (:NewEnumerator0
      (Components|StaticMesh|SetStaticMesh (Variables|Default|GetSM_MoneyBag) "/Game/GA/Meshes/Static_mesh/SM_Pile_Coin.SM_Pile_Coin")
      (Variables|Default|SetMoneyValue 100))
    (:NewEnumerator1
      (Components|StaticMesh|SetStaticMesh (Variables|Default|GetSM_MoneyBag) "/Game/GA/Meshes/Static_mesh/SM_Liasse_Bill.SM_Liasse_Bill")
      (Variables|Default|SetMoneyValue 300))
    (:NewEnumerator2
      (Components|StaticMesh|SetStaticMesh (Variables|Default|GetSM_MoneyBag) "/Game/GA/Meshes/Static_mesh/SM_MoneyBag.SM_MoneyBag")
      (Variables|Default|SetMoneyValue 500))))